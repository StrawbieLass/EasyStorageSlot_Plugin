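; BP_Extinguisher is a held fire extinguisher item that sprays foam and sends extinguish messages to actors.
; A looping fast timer checks the owner's Easy_StorageComponent and destroys the actor if it is no longer the held item.
; While Using, it spawns Niagara foam at the nozzle and sends ExtinguishMessage via a debug-drawn, downward-angled forward trace from the owner.
; SprayArea overlaps also send the message, at higher damage.
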(event OnComponentBeginOverlap(sprayArea)
  (params (OverlappedComponent :type Primitive%20Component%20Object%20Reference) (OtherActor :type Actor%20Object%20Reference) (OtherComp :type Primitive%20Component%20Object%20Reference) (OtherBodyIndex :type Integer) (bFromSweep :type Boolean) (SweepResult :type Hit%20Result%20Structure%20%28by%20ref%29))
  (if (stale EventUseItem using)
    (Class|ItemUsage|Extinguish(Message) OtherActor OtherActor 1.0)))

(event Custom|Held
  (bind _returnvalue (Components|GetOwner))
  (bind _returnvalue_2 (Components|GetOwner))
  (bind _nozzle (Variables|Default|GetNozzle))
  (bind _returnvalue_3 (Actor|GetComponentbyClass _returnvalue "/EasyStorageSlot/Easy_StorageComponent.Easy_StorageComponent_C"))
  (bind _returnvalue_4 (Transformation|GetActorLocation _returnvalue_2))
  (Utilities|IsValid _returnvalue_3
    (:Is%20Valid
      (if (== (.heldobject (Variables|/EasyStorageSlot/Easy_StorageComponent.Easy_StorageComponent_C|GetheldItem _returnvalue_3)) (Utilities|GetClass self))
        (if (stale EventUseItem using)
          (Niagara|SpawnSystematLocation "/EasyStorageSlot/BaseItems/AdvancedBlueprints/FireExtinguisher/NS_Foam.NS_Foam" (Transformation|GetWorldLocation _nozzle) (Transformation|GetWorldRotation _nozzle))
          (bind _outhit (Collision|LineTraceByChannel _returnvalue_4 (+ _returnvalue_4 (* (Transformation|GetActorForwardVector _returnvalue_2) (Math|Float|MakeLiteralFloat 5e+02)) "0.000000,0.000000,-200.000000") "TraceTypeQuery1" false 0 "ForOneFrame"))
          (Class|ItemUsage|Extinguish(Message) (.HitActor (Collision|BreakHitResult _outhit)) (Components|GetOwner) 0.1))
        (else
          (Actor|DestroyActor))))))

(event EventBeginPlay
  (Utilities|Time|SetTimerbyEvent (delegate Custom|Held) 0.01 true))

(event EventUseItem
  (params (using :type Boolean)))

(event EventTick
  (params (DeltaSeconds :type Float%20%28single-precision%29)))

(fn ConstructionScript)